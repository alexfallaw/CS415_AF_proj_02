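; BP_TunnelSpawner builds the endless tunnel, chaining each BP_Tunnel segment from the newest one's SpawnPoint.
; On BeginPlay it clears existing tunnels, enemies, lives and projectiles, then seeds a short chain starting at the player pawn.
; Each segment gets a back-reference to the spawner, a randomized wall, and weighted chances of a life and an enemy.
; Those spawns are scattered forward along X and within a radius in Y/Z.
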(event `self.ReceiveBeginPlay`
  (`self.SpawnInitialTunnels`))

(fn `RandomizePosition`
  (params (Origin :type "Vector Structure"))
  (returns (Position :type "Vector Structure"))
  (locals (R :type "Float (double-precision)") (Theta :type "Float (double-precision)"))
  (bind _returnvalue (* (* (`KismetMathLibrary.GetPI`) 2.0) (`KismetMathLibrary.RandomFloatInRange` 0.0 1.0)))
  (bind _returnvalue_2 (* (`self.Radius`) (`KismetMathLibrary.Sqrt` (`KismetMathLibrary.RandomFloatInRange` 0.0 1.0))))
  (return (`KismetMathLibrary.MakeVector` (+ (`KismetMathLibrary.RandomFloatInRange` (`self.MinDist`) (`self.MaxDist`)) (.x Origin)) (+ (.y Origin) (* _returnvalue_2 (`KismetMathLibrary.Sin` _returnvalue))) (+ (.z Origin) (* _returnvalue_2 (`KismetMathLibrary.Cos` _returnvalue))))))

(fn `SpawnEnemy`
  (params (Origin :type "Vector Structure"))
  (bind _position (`self.RandomizePosition` Origin))
  (`|SpawnActorFromClass` "/Game/InfiniteMatrix/Blueprints/BP_Enemy.BP_Enemy_C" (`KismetMathLibrary.MakeTransform` _position) "AlwaysSpawn" "MultiplyWithRoot" null null))

(fn `SpawnInitialTunnels`
  (`|ExecutionSequence`
    (:`then_0`
      (`|ExecutionSequence`
        (:`then_0`
          (bind _outactors (`GameplayStatics.GetAllActorsOfClass` "/Game/InfiniteMatrix/Blueprints/BP_Tunnel.BP_Tunnel_C"))
          (for _array_element _outactors
            (`self.K2_DestroyActor` _array_element)))
        (:`then_1`
          (bind _outactors_2 (`GameplayStatics.GetAllActorsOfClass` "/Game/InfiniteMatrix/Blueprints/BP_Enemy.BP_Enemy_C"))
          (for _array_element_2 _outactors_2
            (`self.K2_DestroyActor` _array_element_2)))
        (:`then_2`
          (bind _outactors_3 (`GameplayStatics.GetAllActorsOfClass` "/Game/InfiniteMatrix/Blueprints/BP_Life.BP_Life_C"))
          (for _array_element_3 _outactors_3
            (`self.K2_DestroyActor` _array_element_3)))
        (:`then_3`
          (bind _outactors_4 (`GameplayStatics.GetAllActorsOfClass` "/Game/InfiniteMatrix/Blueprints/BP_Projectile.BP_Projectile_C"))
          (for _array_element_4 _outactors_4
            (`self.K2_DestroyActor` _array_element_4)))))
    (:`then_1`
      (for _ (range 3)
        (`/Engine/EditorBlueprintResources/StandardMacros.IsValid` (`self.NewestTunnel`)
          (:`Is Valid`
            (`self.SpawnTunnelAtSpawnPoint`))
          (:`Is Not Valid`
            (`self.SpawnTunnel` (`self.K2_GetActorLocation` (`GameplayStatics.GetPlayerPawn` 0)))))))))

(fn `SpawnLife`
  (params (Origin :type "Vector Structure"))
  (bind _position (`self.RandomizePosition` Origin))
  (`|SpawnActorFromClass` "/Game/InfiniteMatrix/Blueprints/BP_Life.BP_Life_C" (`KismetMathLibrary.MakeTransform` _position) "AlwaysSpawn" "MultiplyWithRoot" null null))

(fn `SpawnTunnel`
  (params (SpawnLocation :type "Vector Structure"))
  (`|ExecutionSequence`
    (:`then_0`
      (bind _returnvalue (`|SpawnActorFromClass` "/Game/InfiniteMatrix/Blueprints/BP_Tunnel.BP_Tunnel_C" (`KismetMathLibrary.MakeTransform` SpawnLocation) "AlwaysSpawn" "MultiplyWithRoot" null null))
      (bind _output_get (set `self.NewestTunnel` _returnvalue))
      (set `/Game/InfiniteMatrix/Blueprints/BP_Tunnel.TunnelSpawner` self _output_get)
      (`/Game/InfiniteMatrix/Blueprints/BP_Tunnel.RandomizeWall` _output_get))
    (:`then_1`
      (if (`KismetMathLibrary.RandomBoolWithWeight` 0.3)
        (`self.SpawnLife` SpawnLocation)))
    (:`then_2`
      (if (`KismetMathLibrary.RandomBoolWithWeight` 0.6)
        (`self.SpawnEnemy` SpawnLocation)))))

(fn `SpawnTunnelAtSpawnPoint`
  (`self.SpawnTunnel` (`SceneComponent.K2_GetComponentLocation` (`/Game/InfiniteMatrix/Blueprints/BP_Tunnel.SpawnPoint` (`self.NewestTunnel`)))))

(fn `UserConstructionScript`)