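; BP_Projectile is a player-scoring projectile that destroys BP_Enemy actors on contact.
; Each tick it sweeps forward along world X at a base speed plus the player's current PlayerSpeed.
; The Cube's hit event destroys a struck enemy, adds score to BP_Player, then destroys the projectile.
; Hits on the player are ignored, while any other hit simply destroys the projectile.
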(event `self.ReceiveTick`
  (params (DeltaSeconds :type "Float (single-precision)"))
  (bind _asbp_player (cast `/Game/InfiniteMatrix/Blueprints/BP_Player` (`GameplayStatics.GetPlayerPawn` 0)))
  (`self.K2_AddActorWorldOffset` (`KismetMathLibrary.MakeVector` (* DeltaSeconds (+ 3000.0 (`/Game/InfiniteMatrix/Blueprints/BP_Player.PlayerSpeed` _asbp_player)))) true))

(event `self.Cube.OnComponentHit`
  (params (HitComponent :type "PrimitiveComponent Object Reference") (OtherActor :type "Actor Object Reference") (OtherComp :type "PrimitiveComponent Object Reference") (NormalImpulse :type "Vector Structure") (Hit :type "HitResult Structure (by ref)"))
  (bind _asbp_enemy (cast `/Game/InfiniteMatrix/Blueprints/BP_Enemy` OtherActor)
    (:`then`
      (`self.K2_DestroyActor` _asbp_enemy)
      (bind _asbp_player (cast `/Game/InfiniteMatrix/Blueprints/BP_Player` (`GameplayStatics.GetPlayerPawn` 0)))
      (set `/Game/InfiniteMatrix/Blueprints/BP_Player.Score` (+ (`/Game/InfiniteMatrix/Blueprints/BP_Player.Score` _asbp_player) 50) _asbp_player))
    (:`CastFailed`
      (cast `/Game/InfiniteMatrix/Blueprints/BP_Player` OtherActor
        (:`CastFailed`
          _))))
  (`self.K2_DestroyActor`))

(fn `UserConstructionScript`)